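; Circus lamp set piece with four player-switchable lamps that reveal a sequence of posed, animated wooden puppets.
; Per-lamp outer and inner spheres swap prompt icons, with the inner one arming its LightSwitch event, which also requires BP_BaseCharacter's IsWatching.
; Switches play lamp animation and sounds, FlipFlop the light, and show their puppet while hiding the previous one.
; Lamp four's DoOnce limits it to one timed puppet jump sequence, ending by revealing SwitchLine.
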(event `Light Switch1`
  (bind _lamp_light1 (`self.Lamp Light1`))
  ; Switch1
  (if (`self.Can Switch1`)
    (bind _returnvalue (`GameplayStatics.GetActorOfClass` "/Game/FirstPerson/Character/Blueprints/BP_BaseCharacter.BP_BaseCharacter_C"))
    (if (`/Game/FirstPerson/Character/Blueprints/BP_BaseCharacter.isWatching?` _returnvalue)
      (`SkeletalMeshComponent.PlayAnimation` (`self.Circus_Lamp_animation`) "/Game/Object/Lamp/Circus_Lamp_animation_Anim.Circus_Lamp_animation_Anim" false)
      (`GameplayStatics.PlaySoundAtLocation` "/Game/music/四顆燈.四顆燈" (`self.K2_GetActorLocation` (`self.fourlightactor`)) (struct) 1.0 1.0 0.0 null null null null)
      (`GameplayStatics.PlaySoundAtLocation` "/Game/music/lampstringonoff38279mp3.lampstringonoff38279mp3" (`SceneComponent.K2_GetComponentLocation` (`self.Lamp1`)) (struct) 1.0 1.0 0.0 null null null null)
      (`/Engine/EditorBlueprintResources/StandardMacros.FlipFlop`
        (:`A`
          (`SkeletalMeshComponent.PlayAnimation` (`self.Wood_Puppet1`) "/Game/Object/WoodPuppet/Pos/Pose7Wood_Puppetˊ_Anim_Armature_025_Action_004.Pose7Wood_Puppetˊ_Anim_Armature_025_Action_004" false)
          (`SceneComponent.SetVisibility` _lamp_light1 true false)
          (`SceneComponent.SetVisibility` (`self.Wood_Puppet1`) true false)
          (`SceneComponent.SetVisibility` (`self.SpotLight1`) true false))
        (:`B`
          (`SceneComponent.SetVisibility` _lamp_light1 false false))))))

(event `self.ReceiveBeginPlay`)

(event `self.ReceiveTick`
  (params (DeltaSeconds :type "Float (single-precision)")))

(event `Light Switch2`
  (bind _lamp_light2 (`self.Lamp Light2`))
  ; Switch2
  (if (`self.Can Switch2`)
    (bind _returnvalue (`GameplayStatics.GetActorOfClass` "/Game/FirstPerson/Character/Blueprints/BP_BaseCharacter.BP_BaseCharacter_C"))
    (if (`/Game/FirstPerson/Character/Blueprints/BP_BaseCharacter.isWatching?` _returnvalue)
      (`SkeletalMeshComponent.PlayAnimation` (`self.Circus_Lamp_animation2`) "/Game/Object/Lamp/Circus_Lamp_animation_Anim.Circus_Lamp_animation_Anim" false)
      (`GameplayStatics.PlaySoundAtLocation` "/Game/music/lampstringonoff38279mp3.lampstringonoff38279mp3" (`SceneComponent.K2_GetComponentLocation` (`self.Lamp2`)) (struct) 1.0 1.0 0.0 null null null null)
      (`GameplayStatics.PlaySoundAtLocation` "/Game/music/四顆燈.四顆燈" (`self.K2_GetActorLocation` (`self.fourlightactor`)) (struct) 1.0 1.0 0.0 null null null null)
      (`/Engine/EditorBlueprintResources/StandardMacros.FlipFlop`
        (:`A`
          (`SceneComponent.SetVisibility` _lamp_light2 true false)
          (`SceneComponent.SetVisibility` (`self.Wood_Puppet2`) true false)
          (`SkeletalMeshComponent.PlayAnimation` (`self.Wood_Puppet2`) "/Game/Object/WoodPuppet/Pos/Pose7Wood_Puppetˊ_Anim_Armature_025_Action_002.Pose7Wood_Puppetˊ_Anim_Armature_025_Action_002" false)
          (`SceneComponent.SetVisibility` (`self.Wood_Puppet1`) false false))
        (:`B`
          (`SceneComponent.SetVisibility` _lamp_light2 false false))))))

(event `Light Switch3`
  (bind _lamp_light3 (`self.Lamp Light3`))
  ; Switch3
  (if (`self.Can Switch3`)
    (bind _returnvalue (`GameplayStatics.GetActorOfClass` "/Game/FirstPerson/Character/Blueprints/BP_BaseCharacter.BP_BaseCharacter_C"))
    (if (`/Game/FirstPerson/Character/Blueprints/BP_BaseCharacter.isWatching?` _returnvalue)
      (`SkeletalMeshComponent.PlayAnimation` (`self.Circus_Lamp_animation3`) "/Game/Object/Lamp/Circus_Lamp_animation_Anim.Circus_Lamp_animation_Anim" false)
      (`GameplayStatics.PlaySoundAtLocation` "/Game/music/lampstringonoff38279mp3.lampstringonoff38279mp3" (`SceneComponent.K2_GetComponentLocation` (`self.Lamp3`)) (struct) 1.0 1.0 0.0 null null null null)
      (`GameplayStatics.PlaySoundAtLocation` "/Game/music/四顆燈.四顆燈" (`self.K2_GetActorLocation` (`self.fourlightactor`)) (struct) 1.0 1.0 0.0 null null null null)
      (`/Engine/EditorBlueprintResources/StandardMacros.FlipFlop`
        (:`A`
          (`SceneComponent.SetVisibility` _lamp_light3 true false)
          (`SceneComponent.SetVisibility` (`self.Wood_Puppet3`) true false)
          (`SkeletalMeshComponent.PlayAnimation` (`self.Wood_Puppet3`) "/Game/Object/WoodPuppet/Pos/Pose7Wood_Puppetˊ_Anim_Armature_025_Action_005.Pose7Wood_Puppetˊ_Anim_Armature_025_Action_005" false)
          (`SceneComponent.SetVisibility` (`self.Wood_Puppet2`) false false))
        (:`B`
          (`SceneComponent.SetVisibility` _lamp_light3 false false))))))

(event `Light Switch4`
  (bind _lamp_light4 (`self.Lamp Light4`))
  (bind _wood_puppet4 (`self.Wood_Puppet4`))
  (bind _switch_line (`self.Switch Line`))
  (bind _wood_puppet4_2 (`self.Wood_Puppet4-2`))
  ; Switch4
  (if (`self.Can Switch4`)
    (bind _returnvalue (`GameplayStatics.GetActorOfClass` "/Game/FirstPerson/Character/Blueprints/BP_BaseCharacter.BP_BaseCharacter_C"))
    (if (`/Game/FirstPerson/Character/Blueprints/BP_BaseCharacter.isWatching?` _returnvalue)
      (`SkeletalMeshComponent.PlayAnimation` (`self.Circus_Lamp_animation4`) "/Game/Object/Lamp/Circus_Lamp_animation_Anim.Circus_Lamp_animation_Anim" false)
      (`GameplayStatics.PlaySoundAtLocation` "/Game/music/lampstringonoff38279mp3.lampstringonoff38279mp3" (`SceneComponent.K2_GetComponentLocation` (`self.Lamp Light4`)) (struct) 1.0 1.0 0.0 null null null null)
      (`GameplayStatics.PlaySoundAtLocation` "/Game/music/四顆燈.四顆燈" (`self.K2_GetActorLocation` (`self.fourlightactor`)) (struct) 1.0 1.0 0.0 null null null null)
      (`/Engine/EditorBlueprintResources/StandardMacros.DoOnce` false
        (:`Completed`
          (`GameplayStatics.PlaySoundAtLocation` "/Game/music/bonge_jumping.bonge_jumping" (`self.K2_GetActorLocation` (`self.fourlightactor`)) (struct) 1.0 1.0 0.0 null null null null)
          (`/Engine/EditorBlueprintResources/StandardMacros.FlipFlop`
            (:`A`
              (`SceneComponent.SetVisibility` _lamp_light4 true false)
              (`SceneComponent.SetVisibility` _wood_puppet4 true false)
              (`SceneComponent.SetVisibility` (`self.Wood_Puppet3`) false false)
              (`SkeletalMeshComponent.PlayAnimation` _wood_puppet4 "/Game/Object/WoodPuppet/Wood_Puppet_-_ˊ_Anim_Armature_022_Armature_022Action_004.Wood_Puppet_-_ˊ_Anim_Armature_022_Armature_022Action_004" false)
              (`KismetSystemLibrary.Delay` 2.0)
              (`SceneComponent.SetVisibility` _wood_puppet4_2 true false)
              (`KismetSystemLibrary.Delay` 0.2)
              (`SceneComponent.SetVisibility` _wood_puppet4 false false)
              (`SkeletalMeshComponent.PlayAnimation` _wood_puppet4_2 "/Game/Object/WoodPuppet/Wood_Puppet_-_ˊ_Anim_Empty_007_Empty_007Action_001.Wood_Puppet_-_ˊ_Anim_Empty_007_Empty_007Action_001" false)
              (`KismetSystemLibrary.Delay` 1.5)
              (`SceneComponent.SetVisibility` _wood_puppet4_2 false false)
              (`SceneComponent.SetVisibility` _switch_line true false)
              (`SkeletalMeshComponent.PlayAnimation` _switch_line "/Game/Object/WoodPuppet/Wood_Puppet_-_ˊ_Anim_Armature_026_Armature_026Action.Wood_Puppet_-_ˊ_Anim_Armature_026_Armature_026Action" false))
            (:`B`
              (`SceneComponent.SetVisibility` _lamp_light4 false false))))))))

(event `self.Inner Sphere Collision1.OnComponentBeginOverlap`
  (params (OverlappedComponent :type "PrimitiveComponent Object Reference") (OtherActor :type "Actor Object Reference") (OtherComp :type "PrimitiveComponent Object Reference") (OtherBodyIndex :type Integer) (bFromSweep :type Boolean) (SweepResult :type "HitResult Structure (by ref)"))
  ; Inner 1
  (if (== OtherActor (`GameplayStatics.GetPlayerCharacter` 0))
    (set `self.Can Switch1` true)
    (`SceneComponent.SetVisibility` (`self.Inner Icon1`) true false)
    (`SceneComponent.SetVisibility` (`self.Outer Icon1`) false false)))

(event `self.Inner Sphere Collision1.OnComponentEndOverlap`
  (params (OverlappedComponent :type "PrimitiveComponent Object Reference") (OtherActor :type "Actor Object Reference") (OtherComp :type "PrimitiveComponent Object Reference") (OtherBodyIndex :type Integer))
  ; Inner 1
  (if (== (`GameplayStatics.GetPlayerCharacter` 0) OtherActor)
    (set `self.Can Switch1` false)
    (`SceneComponent.SetVisibility` (`self.Inner Icon1`) false false)
    (`SceneComponent.SetVisibility` (`self.Outer Icon1`) true false)))

(event `self.Outer Sphere Collision1.OnComponentBeginOverlap`
  (params (OverlappedComponent :type "PrimitiveComponent Object Reference") (OtherActor :type "Actor Object Reference") (OtherComp :type "PrimitiveComponent Object Reference") (OtherBodyIndex :type Integer) (bFromSweep :type Boolean) (SweepResult :type "HitResult Structure (by ref)"))
  ; Outer 1
  (if (== OtherActor (`GameplayStatics.GetPlayerCharacter` 0))
    (`SceneComponent.SetVisibility` (`self.Outer Icon1`) true false)))

(event `self.Outer Sphere Collision1.OnComponentEndOverlap`
  (params (OverlappedComponent :type "PrimitiveComponent Object Reference") (OtherActor :type "Actor Object Reference") (OtherComp :type "PrimitiveComponent Object Reference") (OtherBodyIndex :type Integer))
  ; Outer 1
  (if (== (`GameplayStatics.GetPlayerCharacter` 0) OtherActor)
    (`SceneComponent.SetVisibility` (`self.Outer Icon1`) false false)))

(event `self.Inner Sphere Collision2.OnComponentBeginOverlap`
  (params (OverlappedComponent :type "PrimitiveComponent Object Reference") (OtherActor :type "Actor Object Reference") (OtherComp :type "PrimitiveComponent Object Reference") (OtherBodyIndex :type Integer) (bFromSweep :type Boolean) (SweepResult :type "HitResult Structure (by ref)"))
  ; Inner 2
  (if (== OtherActor (`GameplayStatics.GetPlayerCharacter` 0))
    (set `self.Can Switch2` true)
    (`SceneComponent.SetVisibility` (`self.Inner Icon2`) true false)
    (`SceneComponent.SetVisibility` (`self.Outer Icon2`) false false)))

(event `self.Inner Sphere Collision2.OnComponentEndOverlap`
  (params (OverlappedComponent :type "PrimitiveComponent Object Reference") (OtherActor :type "Actor Object Reference") (OtherComp :type "PrimitiveComponent Object Reference") (OtherBodyIndex :type Integer))
  ; Inner 2
  (if (== (`GameplayStatics.GetPlayerCharacter` 0) OtherActor)
    (set `self.Can Switch2` false)
    (`SceneComponent.SetVisibility` (`self.Inner Icon2`) false false)
    (`SceneComponent.SetVisibility` (`self.Outer Icon2`) true false)))

(event `self.Outer Sphere Collision2.OnComponentBeginOverlap`
  (params (OverlappedComponent :type "PrimitiveComponent Object Reference") (OtherActor :type "Actor Object Reference") (OtherComp :type "PrimitiveComponent Object Reference") (OtherBodyIndex :type Integer) (bFromSweep :type Boolean) (SweepResult :type "HitResult Structure (by ref)"))
  ; Outer 2
  (if (== OtherActor (`GameplayStatics.GetPlayerCharacter` 0))
    (`SceneComponent.SetVisibility` (`self.Outer Icon2`) true false)))

(event `self.Outer Sphere Collision2.OnComponentEndOverlap`
  (params (OverlappedComponent :type "PrimitiveComponent Object Reference") (OtherActor :type "Actor Object Reference") (OtherComp :type "PrimitiveComponent Object Reference") (OtherBodyIndex :type Integer))
  ; Outer 2
  (if (== (`GameplayStatics.GetPlayerCharacter` 0) OtherActor)
    (`SceneComponent.SetVisibility` (`self.Outer Icon2`) false false)))

(event `self.Inner Sphere Collision3.OnComponentBeginOverlap`
  (params (OverlappedComponent :type "PrimitiveComponent Object Reference") (OtherActor :type "Actor Object Reference") (OtherComp :type "PrimitiveComponent Object Reference") (OtherBodyIndex :type Integer) (bFromSweep :type Boolean) (SweepResult :type "HitResult Structure (by ref)"))
  ; Inner 3
  (if (== OtherActor (`GameplayStatics.GetPlayerCharacter` 0))
    (set `self.Can Switch3` true)
    (`SceneComponent.SetVisibility` (`self.Inner Icon3`) true false)
    (`SceneComponent.SetVisibility` (`self.Outer Icon3`) false false)))

(event `self.Inner Sphere Collision3.OnComponentEndOverlap`
  (params (OverlappedComponent :type "PrimitiveComponent Object Reference") (OtherActor :type "Actor Object Reference") (OtherComp :type "PrimitiveComponent Object Reference") (OtherBodyIndex :type Integer))
  ; Inner 3
  (if (== (`GameplayStatics.GetPlayerCharacter` 0) OtherActor)
    (set `self.Can Switch3` false)
    (`SceneComponent.SetVisibility` (`self.Inner Icon3`) false false)
    (`SceneComponent.SetVisibility` (`self.Outer Icon3`) true false)))

(event `self.Outer Sphere Collision3.OnComponentBeginOverlap`
  (params (OverlappedComponent :type "PrimitiveComponent Object Reference") (OtherActor :type "Actor Object Reference") (OtherComp :type "PrimitiveComponent Object Reference") (OtherBodyIndex :type Integer) (bFromSweep :type Boolean) (SweepResult :type "HitResult Structure (by ref)"))
  ; Outer 3
  (if (== OtherActor (`GameplayStatics.GetPlayerCharacter` 0))
    (`SceneComponent.SetVisibility` (`self.Outer Icon3`) true false)))

(event `self.Outer Sphere Collision3.OnComponentEndOverlap`
  (params (OverlappedComponent :type "PrimitiveComponent Object Reference") (OtherActor :type "Actor Object Reference") (OtherComp :type "PrimitiveComponent Object Reference") (OtherBodyIndex :type Integer))
  ; Outer 3
  (if (== (`GameplayStatics.GetPlayerCharacter` 0) OtherActor)
    (`SceneComponent.SetVisibility` (`self.Outer Icon3`) false false)))

(event `self.Inner Sphere Collision4.OnComponentBeginOverlap`
  (params (OverlappedComponent :type "PrimitiveComponent Object Reference") (OtherActor :type "Actor Object Reference") (OtherComp :type "PrimitiveComponent Object Reference") (OtherBodyIndex :type Integer) (bFromSweep :type Boolean) (SweepResult :type "HitResult Structure (by ref)"))
  ; Inner 4
  (if (== OtherActor (`GameplayStatics.GetPlayerCharacter` 0))
    (set `self.Can Switch4` true)
    (`SceneComponent.SetVisibility` (`self.Inner Icon4`) true false)
    (`SceneComponent.SetVisibility` (`self.Outer Icon4`) false false)))

(event `self.Inner Sphere Collision4.OnComponentEndOverlap`
  (params (OverlappedComponent :type "PrimitiveComponent Object Reference") (OtherActor :type "Actor Object Reference") (OtherComp :type "PrimitiveComponent Object Reference") (OtherBodyIndex :type Integer))
  ; Inner 4
  (if (== (`GameplayStatics.GetPlayerCharacter` 0) OtherActor)
    (set `self.Can Switch4` false)
    (`SceneComponent.SetVisibility` (`self.Inner Icon4`) false false)
    (`SceneComponent.SetVisibility` (`self.Outer Icon4`) true false)))

(event `self.Outer Sphere Collision4.OnComponentBeginOverlap`
  (params (OverlappedComponent :type "PrimitiveComponent Object Reference") (OtherActor :type "Actor Object Reference") (OtherComp :type "PrimitiveComponent Object Reference") (OtherBodyIndex :type Integer) (bFromSweep :type Boolean) (SweepResult :type "HitResult Structure (by ref)"))
  ; Outer 4
  (if (== OtherActor (`GameplayStatics.GetPlayerCharacter` 0))
    (`SceneComponent.SetVisibility` (`self.Outer Icon4`) true false)))

(event `self.Outer Sphere Collision4.OnComponentEndOverlap`
  (params (OverlappedComponent :type "PrimitiveComponent Object Reference") (OtherActor :type "Actor Object Reference") (OtherComp :type "PrimitiveComponent Object Reference") (OtherBodyIndex :type Integer))
  ; Outer 4
  (if (== (`GameplayStatics.GetPlayerCharacter` 0) OtherActor)
    (`SceneComponent.SetVisibility` (`self.Outer Icon4`) false false)))

(fn `UserConstructionScript`)