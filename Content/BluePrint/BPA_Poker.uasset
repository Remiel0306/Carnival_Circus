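; BPA_Poker is a Blueprint that plays a repeating poker sound sequence, a hit followed by a drop, from the start of play.
; After a short delay, BeginPlay clears the IsPlaySound flag and calls PokerSoundPlay.
; That event sets the flag, plays PokerHitAudio and PokerDropAudio between timed Delays, then clears it and wires back to its start, looping indefinitely without Tick or timers.
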(event `self.ReceiveBeginPlay`
  (`KismetSystemLibrary.Delay` 0.55)
  (set `self.isPlaySound` false)
  (`self.PokerSoundPlay`))

(event `PokerSoundPlay`
  (if (not (`self.isPlaySound`)) :!label _label
    (set `self.isPlaySound` true)
    (`KismetSystemLibrary.Delay` 0.35)
    (`AudioComponent.Play` (`self.Poker Hit Audio`) 0.0)
    (`KismetSystemLibrary.Delay` 0.6)
    (`AudioComponent.Play` (`self.Poker Drop Audio`) 0.0)
    (`KismetSystemLibrary.Delay` 0.8)
    (set `self.isPlaySound` false)
    (goto _label)))

(fn `UserConstructionScript`)