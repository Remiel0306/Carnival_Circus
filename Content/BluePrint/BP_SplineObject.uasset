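; An actor with a configurable mesh that moves along a referenced spline once a BP_BaseCharacter overlaps its trigger box.
; A timeline, with play rate scaled by TimeToComplete, maps its track to distance along the spline and sets the actor's world location, without using spline rotation.
; A DoOnce on the timeline update plays the Death sound shortly after movement first starts.
; The construction script applies ObjectMesh to the Cube component.
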(event `self.Box.OnComponentBeginOverlap`
  (params (OverlappedComponent :type "PrimitiveComponent Object Reference") (OtherActor :type "Actor Object Reference") (OtherComp :type "PrimitiveComponent Object Reference") (OtherBodyIndex :type Integer) (bFromSweep :type Boolean) (SweepResult :type "HitResult Structure (by ref)"))
  (cast `/Game/FirstPerson/Character/Blueprints/BP_BaseCharacter` OtherActor)
  (`self.Move Object`))

(event `self.ReceiveBeginPlay`)

(event `Move Object`
  (bind _spline (`/Game/BluePrint/BP_SplinePath.Spline` (`self.Spline To Follow`)))
  (`TimelineComponent.SetPlayRate` (`self.T_Move`) (/ 1.0 (`self.Time To Complete`)))
  (bind (_direction _move_track) (`Timeline|T_Move`)
    (:`Update`
      (`self.K2_SetActorLocationAndRotation` (`SplineComponent.GetLocationAtDistanceAlongSpline` _spline (`KismetMathLibrary.Lerp` 0.0 (`SplineComponent.GetSplineLength` _spline) _move_track) "World"))
      (`/Engine/EditorBlueprintResources/StandardMacros.DoOnce` false
        (:`Completed`
          (`KismetSystemLibrary.Delay` 0.1)
          (`GameplayStatics.SpawnSoundAtLocation` "/Game/music/death.death" (0.0 0.0 0.0) (struct) 1.5 1.0 0.0 null null))))))

(fn `UserConstructionScript`
  (`StaticMeshComponent.SetStaticMesh` (`self.Cube`) (`self.Object Mesh`)))