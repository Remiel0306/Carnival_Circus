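; BP_SplinePuppet is a scare-style wooden puppet actor that animates and travels along a referenced spline when triggered.
; One overlap box starts a looping swing animation for the player character; another starts movement for any BP_BaseCharacter.
; A timeline, rate-scaled by TimeToComplete, moves it along the spline, plays a death sound once as movement begins, and hides it when finished.
; The construction script assigns configurable body and chin meshes.
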(event `self.Box Collision1.OnComponentBeginOverlap`
  (params (OverlappedComponent :type "PrimitiveComponent Object Reference") (OtherActor :type "Actor Object Reference") (OtherComp :type "PrimitiveComponent Object Reference") (OtherBodyIndex :type Integer) (bFromSweep :type Boolean) (SweepResult :type "HitResult Structure (by ref)"))
  (if (== OtherActor (`GameplayStatics.GetPlayerCharacter` 0))
    (`SkeletalMeshComponent.PlayAnimation` (`self.Wood_Puppet_swin_new`) "/Game/Object/Hanging_puppet/Wood_Puppet_swin_new_Anim.Wood_Puppet_swin_new_Anim" true)))

(event `self.Box Collision.OnComponentBeginOverlap`
  (params (OverlappedComponent :type "PrimitiveComponent Object Reference") (OtherActor :type "Actor Object Reference") (OtherComp :type "PrimitiveComponent Object Reference") (OtherBodyIndex :type Integer) (bFromSweep :type Boolean) (SweepResult :type "HitResult Structure (by ref)"))
  (cast `/Game/FirstPerson/Character/Blueprints/BP_BaseCharacter` OtherActor)
  (`self.Move Object`))

(event `Move Object`
  (bind _spline (`/Game/BluePrint/BP_SplinePath.Spline` (`self.Spline To Follow`)))
  (`TimelineComponent.SetPlayRate` (`self.Timeline`) (/ 1.0 (`self.Time To Complete`)))
  (bind (_direction _move_track) (`Timeline|Timeline`)
    (:`Update`
      (`self.K2_SetActorLocationAndRotation` (`SplineComponent.GetLocationAtDistanceAlongSpline` _spline (`KismetMathLibrary.Lerp` 0.0 (`SplineComponent.GetSplineLength` _spline) _move_track) "World"))
      (`/Engine/EditorBlueprintResources/StandardMacros.DoOnce` false
        (:`Completed`
          (`GameplayStatics.SpawnSoundAtLocation` "/Game/music/death.death" (0.0 0.0 0.0) (struct) 1.5 1.0 0.0 null null))))
    (:`Finished`
      (`self.SetActorHiddenInGame` true))))

(fn `UserConstructionScript`
  (`StaticMeshComponent.SetStaticMesh` (`self.Body_024`) (`self.New Mesh_0`))
  (`StaticMeshComponent.SetStaticMesh` (`self.Chin_016`) (`self.New Mesh`)))