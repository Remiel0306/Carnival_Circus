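; Audio controller Blueprint that shifts a soundscape from crying to laughter as overlaps occur on trigger components.
; SoundControl loops the first cry on timed Delays until the first trigger is touched, then alternates both cries until the second trigger stops them.
; The triggers also start environment audio and a buffered transition into laughter, while AllStop silences these main sounds.
; The first cry's finished callback sets a flag that is never read here.
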(event `self.ReceiveBeginPlay`
  (`self.Sound Control`)
  (add `AudioComponent.OnAudioFinished` (`self.First Cry Audio`) (delegate `Handle First Cry Finished`))
  (`AudioComponent.Play` (`self.First Cry Audio`) 0.0))

(event `Handle First Cry Finished`
  (set `self.IsFirstCryFinish?` true))

(event `Sound Control`
  (`AudioComponent.Play` (`self.First Cry Audio`) 0.0 :!label _label)
  (`KismetSystemLibrary.Delay` 11.0)
  (if (`self.IsTouchFirst?`)
    (`KismetSystemLibrary.PrintString` "1")
    (`AudioComponent.Play` (`self.Second Cry Audio`) 0.0 :!label _label_2)
    (`KismetSystemLibrary.Delay` 8.0)
    (`AudioComponent.Play` (`self.First Cry Audio`) 0.0)
    (`KismetSystemLibrary.Delay` 11.0)
    (if (`self.IsTouchSecond?`)
      (`KismetSystemLibrary.Delay` 3.0)
      (`AudioComponent.Stop` (`self.First Cry Audio`))
      (`AudioComponent.Stop` (`self.Second Cry Audio`))
      (else
        (goto _label_2)))
    (else
      (goto _label))))

(event `self.First to Second.OnComponentBeginOverlap`
  (params (OverlappedComponent :type "PrimitiveComponent Object Reference") (OtherActor :type "Actor Object Reference") (OtherComp :type "PrimitiveComponent Object Reference") (OtherBodyIndex :type Integer) (bFromSweep :type Boolean) (SweepResult :type "HitResult Structure (by ref)"))
  (set `self.IsTouchFirst?` true)
  (`AudioComponent.Play` (`self.Environment Auido`) 0.0))

(event `self.Second to Third .OnComponentBeginOverlap`
  (params (OverlappedComponent :type "PrimitiveComponent Object Reference") (OtherActor :type "Actor Object Reference") (OtherComp :type "PrimitiveComponent Object Reference") (OtherBodyIndex :type Integer) (bFromSweep :type Boolean) (SweepResult :type "HitResult Structure (by ref)"))
  (set `self.IsTouchSecond?` true)
  (`AudioComponent.Play` (`self.Cry to Lough Buffer Audio`) 0.0)
  (`KismetSystemLibrary.Delay` 3.0)
  (`AudioComponent.Play` (`self.Laugh Audio`) 0.0))

(event `self.All Stop.OnComponentBeginOverlap`
  (params (OverlappedComponent :type "PrimitiveComponent Object Reference") (OtherActor :type "Actor Object Reference") (OtherComp :type "PrimitiveComponent Object Reference") (OtherBodyIndex :type Integer) (bFromSweep :type Boolean) (SweepResult :type "HitResult Structure (by ref)"))
  (`AudioComponent.Stop` (`self.Environment Auido`))
  (`AudioComponent.Stop` (`self.Laugh Audio`))
  (`AudioComponent.Stop` (`self.First Cry Audio`))
  (`AudioComponent.Stop` (`self.Second Cry Audio`)))

(fn `UserConstructionScript`)