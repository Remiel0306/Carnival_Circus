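; BPA_PuppetRun is an actor that slides a puppet across the level when the player walks into its trigger.
; At BeginPlay it caches the world positions of two referenced marker actors as start and end points.
; On player overlap, a timeline drives a lerp between those points and sets the puppet's world location each update, without sweep.
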(event `self.ReceiveBeginPlay`
  (set `self.StartLocation` (`self.K2_GetActorLocation` (`self.actorStartLocation`)))
  (set `self.EndLoction` (`self.K2_GetActorLocation` (`self.actorEndLocation`))))

(event `self.Trigger.OnComponentBeginOverlap`
  (params (OverlappedComponent :type "PrimitiveComponent Object Reference") (OtherActor :type "Actor Object Reference") (OtherComp :type "PrimitiveComponent Object Reference") (OtherBodyIndex :type Integer) (bFromSweep :type Boolean) (SweepResult :type "HitResult Structure (by ref)"))
  (if (== OtherActor (`GameplayStatics.GetPlayerCharacter` 0))
    (bind (_direction _puppet_run) (`Timeline|Run`)
      (:`Update`
        (`SceneComponent.K2_SetWorldLocation` (`self.Puppet`) (`KismetMathLibrary.VLerp` (`self.StartLocation`) (`self.EndLoction`) _puppet_run) false false)))))

(fn `UserConstructionScript`)