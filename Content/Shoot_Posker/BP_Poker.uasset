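; BP_Poker is a poker card Blueprint whose only logic plays a repeating card hit and drop sound sequence.
; After a short delay on BeginPlay, PokerSoundPlay chains timed delays with 2D sound playback, then clears its IsPlaySound guard and loops back indefinitely.
; Location-based versions of both sounds remain in the graph but are disconnected.
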(event `self.ReceiveBeginPlay`
  (`KismetSystemLibrary.Delay` 0.55)
  (set `self.isPlaySound` false)
  (`self.PokerSoundPlay`))

(event `PokerSoundPlay`
  (if (not (`self.isPlaySound`)) :!label _label
    (set `self.isPlaySound` true)
    (`KismetSystemLibrary.Delay` 0.35)
    (`GameplayStatics.PlaySound2D` "/Game/SoundEffect/Poker/SW_Poker_card_hit.SW_Poker_card_hit" 1.0 1.0 0.0 null null)
    (`KismetSystemLibrary.Delay` 0.65)
    (`GameplayStatics.PlaySound2D` "/Game/SoundEffect/Poker/SW_Poker_card_drop.SW_Poker_card_drop" 1.0 1.0 0.0 null null)
    (`KismetSystemLibrary.Delay` 0.8)
    (set `self.isPlaySound` false)
    (goto _label)))

(fn `UserConstructionScript`)